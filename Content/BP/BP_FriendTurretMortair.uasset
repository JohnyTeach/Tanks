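; Friendly mortar turret Blueprint whose live event graph only turns its HP bar toward the player camera every tick.
; Helper functions select the nearest enemy-tagged actor, rotate the turret toward it in yaw only and call Fire within AttackRadius.
; That Blueprint firing routine and the targeting-sphere radius setup are disconnected in the event graph, so neither runs from there.
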(event `self.ReceiveBeginPlay`
  ;[1 1 1] Установка радиуса для стрельбы турелли
)

(event `self.ReceiveTick`
  (params (DeltaSeconds :type "Float (single-precision)"))
  (bind _hpbar (`self.HPBar`))
  ;[1 1 1] Поворот HP бара за камерой игрока
  (`SceneComponent.K2_SetWorldRotation` _hpbar (`KismetMathLibrary.FindLookAtRotation` (`SceneComponent.K2_GetComponentLocation` _hpbar) (`PlayerCameraManager.GetCameraLocation` (`GameplayStatics.GetPlayerCameraManager` 0))) false false))

(fn `GetLength`
  (params (Enemy :type "Actor Object Reference"))
  (returns (Lenght :type "Float (double-precision)"))
  ;[1 1 1] Определение расстояния до цели
  (`/Engine/EditorBlueprintResources/StandardMacros.IsValid` Enemy
    (:`Is Valid`
      (return (`KismetMathLibrary.VSize` (- (`SceneComponent.K2_GetComponentLocation` (`self.Turret`)) (`self.K2_GetActorLocation` Enemy)))))))

(fn `SelectEnemy`
  (returns (Enemy :type "Actor Object Reference"))
  (locals (CurrentIndex :type Integer) (MinLength :type "Float (double-precision)"))
  ;[1 1 1] Выбор цели для стрельбы
  (bind _outactors (`GameplayStatics.GetAllActorsWithTag` (`self.EnemyTag`)))
  (bind _output_get (set `self.ArrayEnemy` _outactors))
  (bind _lenght (`self.GetLength` (`|GetArrayItem` _output_get)))
  (set `local.MinLength` _lenght)
  (for _index (range (+ (`KismetArrayLibrary.Array_Length` (`self.ArrayEnemy`)) 1))
    (bind _lenght_2 (`self.GetLength` (`|GetArrayItem` (`self.ArrayEnemy`) _index)))
    (if (< _lenght_2 (`local.MinLength`))
      (set `local.CurrentIndex` _index)
      (set `local.MinLength` _lenght_2)))
  (return (`|GetArrayItem` (`self.ArrayEnemy`) (`local.CurrentIndex`))))

(fn `Turret Fire`
  (bind (_returnvalue_roll _returnvalue_pitch _returnvalue_yaw) (`KismetMathLibrary.BreakRotator` (`KismetMathLibrary.FindLookAtRotation` (`self.TurretLocation`) (`self.EnemyLocation`))))
  ;[1 1 1] Реализация стрельбы по ближайшей цели
  (bind _enemy (`self.SelectEnemy`))
  (`/Engine/EditorBlueprintResources/StandardMacros.IsValid` _enemy
    (:`Is Valid`
      (set `self.EnemyLocation` (`self.K2_GetActorLocation` _enemy))
      (set `self.TurretLocation` (`SceneComponent.K2_GetComponentLocation` (`self.Turret`)))
      (`SceneComponent.K2_SetWorldRotation` (`self.Turret`) (`KismetMathLibrary.MakeRotator` 0.0 0.0 _returnvalue_yaw) false false)
      (if (< (`KismetMathLibrary.VSize` (- (`self.TurretLocation`) (`self.EnemyLocation`))) (`self.AttackRadius`))
        (`self.Fire`)))))

(fn `UserConstructionScript`)